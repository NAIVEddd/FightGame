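; Base weapon Blueprint that shows an interaction prompt while a player is in range.
; On range entry, it creates a SimpleUI widget with the GetShowName text ("Pick Up") in a screen-space, collision-free widget component, if none is valid.
; The component snaps to GetInteractionTextAttach, which returns nothing here, and is destroyed on range exit.
; No pickup logic is implemented here.
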(event `OnInteractionRangeEntered_1`
  (params (Player :type "Soldier Object Reference"))
  (bind _text (`self.GetShowName`))
  (`self.InteractionWidget`
    (:`then`)
    (:`else`
      (bind _returnvalue (`|CreateWidget` "/Game/Enemy/UI/SimpleUI.SimpleUI_C" (cast `PlayerController` (`Pawn.GetController` Player) :!pure true) _text))
      (bind _returnvalue_2 (`AddComponent|NODE_AddWidgetComponent-0`))
      (bind _output_get (set `self.InteractionWidget` _returnvalue_2))
      (`WidgetComponent.SetWidget` _output_get _returnvalue)
      (`WidgetComponent.SetWidgetSpace` _output_get "Screen")
      (`WidgetComponent.SetDrawAtDesiredSize` _output_get true)
      (`PrimitiveComponent.SetCollisionEnabled` _output_get "NoCollision")
      (`SceneComponent.K2_AttachToComponent` _output_get (`self.GetInteractionTextAttach`) "None" "SnapToTarget" "SnapToTarget" "SnapToTarget" true))))

(event `OnInteractionRangeExited_1`
  (bind _interactionwidget (`self.InteractionWidget`)
    (:`then`
      (`ActorComponent.K2_DestroyComponent` _interactionwidget))
    (:`else`)))

(fn `GetInteractionTextAttach`
  (returns (AttachComponent :type "SceneComponent Object Reference"))
  (return null))

(fn `GetShowName`
  (returns (Text :type Text))
  (return "Pick Up"))

(fn `UserConstructionScript`)