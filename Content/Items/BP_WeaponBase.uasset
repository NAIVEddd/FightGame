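; Base weapon actor that a BP_Soldier can pick up, drop and fire.
; Interaction range events create and remove a screen-space pickup prompt, and interacting hands the weapon to the soldier.
; A Dropped/Equipped state switches collision profiles on the sphere and skeletal mesh.
; Fire spawns a projectile and muzzle flash at the muzzle socket, aimed at a point along the player's forward vector, with debug drawing.
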(event `InteractionInterface.OnInteractionRangeEntered`
  (params (Player :type "Soldier Object Reference"))
  (bind _text (`self.GetShowName`))
  (`self.InteractionWidget`
    (:`then`)
    (:`else`
      (bind _returnvalue (`|CreateWidget` "/Game/UI/SimpleUI.SimpleUI_C" (cast `PlayerController` (`Pawn.GetController` Player) :!pure true) _text))
      (bind _returnvalue_2 (`AddComponent|NODE_AddWidgetComponent-0`))
      (bind _output_get (set `self.InteractionWidget` _returnvalue_2))
      (`WidgetComponent.SetWidget` _output_get _returnvalue)
      (`WidgetComponent.SetWidgetSpace` _output_get "Screen")
      (`WidgetComponent.SetDrawAtDesiredSize` _output_get true)
      (`PrimitiveComponent.SetCollisionEnabled` _output_get "NoCollision")
      (`SceneComponent.K2_AttachToComponent` _output_get (`self.GetInteractionTextAttach`) "None" "SnapToTarget" "SnapToTarget" "SnapToTarget" true))))

(event `InteractionInterface.OnInteractionRangeExited`
  (bind _interactionwidget (`self.InteractionWidget`)
    (:`then`
      (`ActorComponent.K2_DestroyComponent` _interactionwidget))
    (:`else`)))

(event `self.ReceiveBeginPlay`
  (`self.SetWeaponState` "NewEnumerator0"))

(event `InteractionInterface.OnInteracted`
  (params (Player :type "Soldier Object Reference"))
  (`KismetSystemLibrary.PrintString` "Hello")
  (bind _asbp_soldier (cast `/Game/Character/Blueprints/BP_Soldier` Player))
  (`/Game/Character/Blueprints/BP_Soldier.PickUpWeapon` _asbp_soldier self)
  (`self.SetWeaponState` "NewEnumerator1"))

(fn `DropWeapon`
  (`self.SetWeaponState` "NewEnumerator0"))

(fn `Fire`
  (params (Player :type "/Game/Character/Blueprints/BP_Soldier Object Reference"))
  (bind _returnvalue (`SceneComponent.GetSocketLocation` (`self.SkeletalMesh`) "b_gun_muzzleflash"))
  (bind _returnvalue_2 (+ (`self.K2_GetActorLocation` Player) (* (`self.GetActorForwardVector` Player) 3000.0)))
  (`KismetSystemLibrary.DrawDebugPoint` _returnvalue_2 10.0 (struct :`R` 0.018 :`G` 1.0 :`B` 0.104 :`A` 1.0) 0.5)
  (`KismetSystemLibrary.DrawDebugLine` _returnvalue _returnvalue_2 (struct) 0.5)
  (`|SpawnActorFromClass` "/Game/Items/Gun/Bullet/BP_Bullet.BP_Bullet_C" (`KismetMathLibrary.MakeTransform` _returnvalue) "Undefined" "OverrideRootScale" null (* (`KismetMathLibrary.Normal` (- _returnvalue_2 _returnvalue)) 10000.0) null)
  (`|SpawnActorFromClass` "/Game/Items/Gun/Bullet/BP_MuzzleFlash.BP_MuzzleFlash_C" (`KismetMathLibrary.MakeTransform` _returnvalue) "Undefined" "OverrideRootScale" null null))

(fn `GetInteractionTextAttach`
  (returns (AttachComponent :type "SceneComponent Object Reference"))
  (return (`self.DefaultSceneRoot`)))

(fn `GetShowName`
  (returns (Text :type Text))
  (return "Pick Up"))

(fn `SetWeaponState`
  (params (WeaponState :type "/Game/Items/Gun/Enum_GunState Enum" :default "NewEnumerator0"))
  (bind _output_get (set `self.WeaponState` WeaponState))
  (switch `/Game/Items/Gun/Enum_GunState` _output_get
    (:`NewEnumerator0`
      (`PrimitiveComponent.SetCollisionProfileName` (`self.Sphere`) "OverlapAllDynamic" true)
      (`PrimitiveComponent.SetCollisionProfileName` (`self.SkeletalMesh`) "DroppedWeapon" true))
    (:`NewEnumerator1`
      (`PrimitiveComponent.SetCollisionProfileName` (`self.Sphere`) "NoCollision" false)
      (`PrimitiveComponent.SetCollisionProfileName` (`self.SkeletalMesh`) "NoCollision" false))))

(fn `UserConstructionScript`)